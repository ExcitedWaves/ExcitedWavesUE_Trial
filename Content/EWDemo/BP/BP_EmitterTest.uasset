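; Test sound emitter actor for an acoustics demo, playing a switchable list of Wwise events.
; BeginPlay posts the current event if enabled, and a looping timer reposts it when IsLoop is set.
; Input actions play, stop, cycle events and mute the dry signal through a volume RTPC.
; Tick feeds AcousticsDetector reverb and room debug data to the player's results widget and optionally moves the emitter in a circle.
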(event Custom|PlayAudio
  (if (Variables|Default|GetisLoop)
    (Utilities|FlowControl|Sequence
      (:then_1
        (if (Variables|Default|GetplaysAudio)
          (Class|AkGameObject|PostAkEvent (Variables|Default|GetAk) (Utilities|Array|Get(acopy) (Variables|Default|GetEvent) (Variables|Default|GetcurAudioIdx))))))))

(event EventBeginPlay
  (Utilities|FlowControl|Sequence
    (:then_0
      (Utilities|Time|SetTimerbyEvent (delegate Custom|PlayAudio) (Variables|Default|GetTimer) true))
    (:then_1
      (Utilities|FlowControl|Sequence
        (:then_1
          (if (Variables|Default|GetplaysAudio)
            (Class|AkGameObject|PostAkEvent (Variables|Default|GetAk) (Utilities|Array|Get(acopy) (Variables|Default|GetEvent) (Variables|Default|GetcurAudioIdx)))))))
    (:then_2
      (Development|ExecuteConsoleCommand "r.Shadow.Virtual.AllowScreenOverflowMessages 0" 0))))

(event EventTick
  (params (DeltaSeconds :type Float%20%28single-precision%29))
  (bind _acousticsdetector (Variables|Default|GetAcousticsDetector))
  (bind _returnvalue (Class|AcousticsDetectorComponent|GetDebugOverlayData _acousticsdetector))
  (Utilities|FlowControl|Sequence
    (:then_0
      (bind _asbp_shooter_character (Utilities|Casting|CastToBP_ShooterCharacter (Pawn|GetControlledPawn (Game|GetPlayerController 0))))
      (Default|SetParameters (Variables|/Game/EWDemo/UI/WBP_AcousticsDebugOverlay.WBP_AcousticsDebugOverlay_C|GetWBP_Values_Emitter (Variables|/Game/Variant_Shooter/Blueprints/BP_ShooterCharacter.BP_ShooterCharacter_C|GetResultsWidget _asbp_shooter_character)) (.close _returnvalue) (.mid _returnvalue) (.far _returnvalue) (.originalclose _returnvalue) (.originalmid _returnvalue) (.originalfar _returnvalue) (.outdoor _returnvalue) (.originaloutdoor _returnvalue) (.absorption _returnvalue) (.bisindoor _returnvalue) (.reverbenclosure _returnvalue) (.height _returnvalue) (.width _returnvalue) (.distancetolistener _returnvalue) (.reverbmultiplier _returnvalue) (.crossroomcontribution _returnvalue) "Emitter Parameters"))
    (:then_1
      (if (Variables|Default|GetisMoving)
        ;[1 1 1] Movement
        (Transformation|SetActorLocation (+ (Transformation|GetActorLocation) (* (Transformation|GetActorForwardVector) (* 9e+02 (* DeltaSeconds 0.3)))) false true)
        (Class|Actor|AddActorWorldRotation (Math|Rotator|MakeRotator 0.0 0.0 (* 45.0 DeltaSeconds)))))))

(event Input|ActionEvents|InputActionMuteDry
  (params (Key :type Key%20Structure :default "None"))
  (:Pressed
    (bind _output_get (Variables|Default|SetmuteDry (not (Variables|Default|GetmuteDry))))
    (if _output_get
      (Class|AkGameObject|SetRTPCValue (Variables|Default|GetAk) "/Game/WwiseAudio/RTPCs/EmitterVolume.EmitterVolume" 0.0)
      (Default|DryWet (Variables|/Game/Variant_Shooter/Blueprints/BP_ShooterCharacter.BP_ShooterCharacter_C|GetResultsWidget (stale EventTick _asbp_shooter_character)) false)
      (else
        (Class|AkGameObject|SetRTPCValue (Variables|Default|GetAk) "/Game/WwiseAudio/RTPCs/EmitterVolume.EmitterVolume" 1e+02)
        (Default|DryWet (Variables|/Game/Variant_Shooter/Blueprints/BP_ShooterCharacter.BP_ShooterCharacter_C|GetResultsWidget (stale EventTick _asbp_shooter_character)) true)))))

(event Input|ActionEvents|InputActionStopPlay
  (params (Key :type Key%20Structure :default "None"))
  (:Pressed
    (Variables|Default|SetplaysAudio false)
    (Class|AkGameObject|Stop (Variables|Default|GetAk))))

(event Input|ActionEvents|InputActionPlay
  (params (Key :type Key%20Structure :default "None"))
  (:Pressed
    (if (not (Variables|Default|GetplaysAudio))
      (Variables|Default|SetplaysAudio true)
      (Class|AkGameObject|PostAkEvent (Variables|Default|GetAk) (Utilities|Array|Get(acopy) (Variables|Default|GetEvent) (Variables|Default|GetcurAudioIdx))))))

(event Input|ActionEvents|InputActionNextAudio
  (params (Key :type Key%20Structure :default "None"))
  (bind _ak (Variables|Default|GetAk))
  (:Pressed
    (Utilities|FlowControl|Sequence
      (:then_0
        (Variables|Default|SetplaysAudio false)
        (Class|AkGameObject|Stop _ak))
      (:then_1
        (bind _result (Math|Integer|IncrementInt (Variables|Default|GetcurAudioIdx))
          (:%20%20
            (bind _output_get (Variables|Default|SetcurAudioIdx _result))
            (if (>= _output_get (Utilities|Array|Length (Variables|Default|GetEvent)))
              (Variables|Default|SetcurAudioIdx 0))
            (Variables|Default|SetplaysAudio true)
            (Class|AkGameObject|PostAkEvent _ak (Utilities|Array|Get(acopy) (Variables|Default|GetEvent) (Variables|Default|GetcurAudioIdx)))))))))

(fn ConstructionScript)

(fn Interact
  (return 0))